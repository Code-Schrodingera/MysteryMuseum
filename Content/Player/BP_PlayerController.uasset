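; Player controller for click-to-move play with item interaction and pickup.
; Left click sends BP_Player to the point under the cursor and stores any interactable BP_ItemBased hit there as the target.
; When the character's target-reached event fires, the controller interacts with that item; the item's picked-up event adds its description to the player's inventory.
; Tick traces under the cursor to highlight interactables.
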(event Custom|PlaceItemToInventory
  (params (ItemRef :type BP%20Item%20Based%20Object%20Reference))
  (bind _asbp_player (Utilities|Casting|CastToBP_Player (Pawn|GetControlledPawn)))
  (Utilities|Array|Add (Variables|/Game/Player/BP_Player.BP_Player_C|GetInventory _asbp_player) (Variables|/Game/Items/BP_ItemBased.BP_ItemBased_C|GetItemDesc ItemRef)))

(event Custom|CharacterReachedTarget
  (bind _targetitem (Variables|Default|GetTargetItem))
  (Utilities|IsValid _targetitem
    (:Is%20Valid
      (Default|Interact _targetitem))))

(event EventTick
  (params (DeltaSeconds :type Float%20%28single-precision%29))
  (bind _hitresult (Game|Player|GetHitResultUnderCursorbyChannel "TraceTypeQuery1" true))
  (if (Utilities|DoesObjectImplementInterface (.hitactor _hitresult) "/Game/Items/BPI_Interactable.BPI_Interactable_C")
    (bind _asbpi_interactable (Utilities|Casting|CastToBPI_Interactable (.hitactor _hitresult)))
    (Default|Highlight _asbpi_interactable)))

(event EventPossess
  (params (PossessedPawn :type Pawn%20Object%20Reference))
  (bind _asbp_player (Utilities|Casting|CastToBP_Player PossessedPawn))
  (EventDispatchers|BindEventtoTargetReached _asbp_player (delegate Custom|CharacterReachedTarget))
  (Variables|Default|SetbShowMouseCursor true))

(event Input|MouseEvents|LeftMouseButton
  (params (Key :type Key%20Structure :default "None"))
  (bind _hitresult (Game|Player|GetHitResultUnderCursorbyChannel "TraceTypeQuery1" true))
  (:Pressed
    (bind _asbp_player (Utilities|Casting|CastToBP_Player (Pawn|GetControlledPawn)))
    (Default|SetNewTarget _asbp_player (.location _hitresult))
    (if (Utilities|DoesObjectImplementInterface (.hitactor _hitresult) "/Game/Items/BPI_Interactable.BPI_Interactable_C")
      (bind _asbp_item_based (Utilities|Casting|CastToBP_ItemBased (.hitactor _hitresult)))
      (bind _output_get (Variables|Default|SetTargetItem _asbp_item_based))
      (EventDispatchers|BindEventtoOnPickedUp _output_get (delegate Custom|PlaceItemToInventory))
      (else
        ;[1 1 1] За-null-яем переменную
        (Variables|Default|SetTargetItem 0)))))

(fn ConstructionScript)