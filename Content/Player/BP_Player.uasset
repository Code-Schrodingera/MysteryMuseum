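; Player Blueprint that moves to a target location through AI navigation and signals when it arrives.
; SetNewTarget stores the goal and starts Simple Move To Location on the controller.
; Tick polls the distance to that goal and calls TargetReached inside AcceptableRadius, repeating every frame while it stays in range.
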(event EventBeginPlay)

(event Collision|EventActorBeginOverlap
  (params (OtherActor :type Actor%20Object%20Reference)))

(event EventTick
  (params (DeltaSeconds :type Float%20%28single-precision%29))
  (if (< (Math|Vector|Distance(Vector) (Variables|Default|GetTargetGoal) (Transformation|GetActorLocation)) (Variables|Default|GetAcceptableRadius))
    (Default|CallTargetReached)))

(fn ConstructionScript)

(fn SetNewTarget
  (params (NewTarget :type Vector))
  (bind _output_get (Variables|Default|SetTargetGoal NewTarget))
  (AI|Navigation|SimpleMovetoLocation (Pawn|GetController) _output_get))