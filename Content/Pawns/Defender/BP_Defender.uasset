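; BP_Defender is a pawn that moves on the navmesh and searches an area for the player.
; Each tick it fires the TargetReached dispatcher while it is within DistanceToKill of TargetPoint.
; ScanningForPlayer makes three timed moves to random reachable points within RandomScanRadius of itself, then fires ScanningIsOver.
; A PlayAnimation event plays a given animation directly on the mesh, optionally looping.
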(event Custom|PlayAnimation
  (params (AnimToPlay :type Anim%20Sequence%20Object%20Reference) (Looping :type Boolean))
  (Components|Animation|PlayAnimation (Variables|Character|GetMesh) AnimToPlay Looping))

(event Custom|ScanningForPlayer
  (bind _returnvalue (Transformation|GetActorLocation))
  (bind _returnvalue_2 (Pawn|GetController))
  (bind _randomscanradius (Variables|Default|GetRandomScanRadius))
  (bind _randomlocation (AI|Navigation|GetRandomReachablePointinRadius _returnvalue _randomscanradius 0 0))
  (AI|Navigation|SimpleMovetoLocation _returnvalue_2 _randomlocation)
  (Utilities|FlowControl|Delay 2.0)
  (AI|Navigation|SimpleMovetoLocation _returnvalue_2 _randomlocation)
  (Utilities|FlowControl|Delay 2.0)
  (AI|Navigation|SimpleMovetoLocation _returnvalue_2 _randomlocation)
  (Utilities|FlowControl|Delay 2.0)
  (Default|CallScanningIsOver))

(event EventTick
  (params (DeltaSeconds :type Float%20%28single-precision%29))
  (if (< (Math|Vector|Distance(Vector) (Variables|Default|GetTargetPoint) (Transformation|GetActorLocation)) (Variables|Default|GetDistanceToKill))
    (Default|CallTargetReached)))

(fn ConstructionScript)