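; AI controller for the Defender enemy that rests, scans, chases and kicks BP_Player dead, or returns to its start point.
; A gameplay-tag state machine runs movement and animations, while AI perception switches it between Alarmed and Aggression states.
; Fuzzy logic decides waking, stopping the chase and attacking, using text-parsed rules over Distance, Awaken and AttackPlayer variables built at BeginPlay.
; BT_Defender also starts on possession, and pawn callbacks advance the scanning and returning states.
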(event InitStateDelegate(StateMachine)
  (params (StateTag :type Gameplay%20Tag%20Structure%20%28by%20ref%29))
  (|SwitchGameplayTag StateTag
    (:Defender.Resting
      (CallFunction|StartResting))
    (:Defender.Aggression.Chasing
      (CallFunction|ChasePlayer))
    (:Defender.Aggression.Attacking
      (CallFunction|KillPlayer))
    (:Defender.Alarmed.RunningToPoint
      (CallFunction|RuntoTarget))
    (:Defender.Alarmed.Scanning
      (Default|ScanningforPlayer (Variables|Default|GetAs%20BP%20Defender)))
    (:Defender.Alarmed.Returning
      (Variables|Default|SetTargetPoint (Variables|Default|GetStartPoint))
      (CallFunction|RuntoTarget))))

(event EndStateDelegate(StateMachine)
  (params (StateTag :type Gameplay%20Tag%20Structure%20%28by%20ref%29))
  (|SwitchGameplayTag StateTag
    (:Defender.Aggression.Attacking
      (Utilities|FlowControl|Delay 2.0))))

(event TickStateDelegate(StateMachine)
  (params (DeltaTime :type Float%20%28single-precision%29) (StateTag :type Gameplay%20Tag%20Structure%20%28by%20ref%29))
  (bind _fengine (Variables|Default|GetFEngine))
  (bind _termselector (Variables|Default|GetTermSelector))
  (Utilities|FlowControl|Delay 0.2)
  (Utilities|FlowControl|Sequence
    (:then_0
      (if (GameplayTags|MatchesTag StateTag "(TagName=\"Defender.Aggression\")")
        (if (not (Variables|Default|GetPlayerVisible))
          (Class|StateMachineComponent|SwitchState (Variables|Default|GetStateMachine) "(TagName=\"Defender.Alarmed.Scanning\")"))))
    (:then_1
      (if (GameplayTags|MatchesTag StateTag "(TagName=\"Defender.Alarmed\")")
        (if (Variables|Default|GetPlayerVisible)
          (Class|StateMachineComponent|SwitchState (Variables|Default|GetStateMachine) "(TagName=\"Defender.Aggression.Chasing\")"))))
    (:then_2
      (|SwitchGameplayTag StateTag
        (:Defender.Resting
          (Utilities|FlowControl|Delay 2.0)
          (bind _returnvalue (Class|FEngine|Evaluate _fengine (Variables|Default|GetRulesToSleep)))
          (switch string (Class|TermSelector|SelectTerm _termselector (Variables|Default|GetAwaken) _returnvalue)
            (:Awaken
              (Class|StateMachineComponent|SwitchState (Variables|Default|GetStateMachine) "(TagName=\"Defender.Alarmed.Scanning\")")
              (Development|PrintString "Bot is Awaken" true true "(R=1.000000,G=0.616509,B=0.000000,A=1.000000)"))))
        (:Defender.Aggression.Chasing
          (Utilities|FlowControl|Sequence
            (:then_0
              (bind _returnvalue_2 (Class|FEngine|Evaluate _fengine (Variables|Default|GetRulesToChase)))
              (switch string (Class|TermSelector|SelectTerm _termselector (Variables|Default|GetAwaken) _returnvalue_2)
                (:NotAwaken
                  (Class|StateMachineComponent|SwitchState (Variables|Default|GetStateMachine) "(TagName=\"Defender.Alarmed.Returning\")")
                  (Development|PrintString "Chasing Stopped" true true "(R=1.000000,G=0.097600,B=0.000000,A=1.000000)"))))
            (:then_1
              (bind _returnvalue_3 (Class|FEngine|Evaluate (Variables|Default|GetFEngine) (Variables|Default|GetRulesToAttack)))
              (switch string (Class|TermSelector|SelectTerm (Variables|Default|GetTermSelector) (Variables|Default|GetAttackPlayer) _returnvalue_3)
                (:Punch
                  (Class|StateMachineComponent|SwitchState (Variables|Default|GetStateMachine) "(TagName=\"Defender.Aggression.Attacking\")")
                  (Development|PrintString "AttackBegin" true true "(R=1.000000,G=0.437420,B=0.000000,A=1.000000)"))))))))))

(event OnTargetPerceptionUpdated(AIPerception)
  (params (Actor :type Actor%20Object%20Reference) (Stimulus :type AI%20Stimulus%20Structure))
  (Utilities|Casting|CastToBP_Player Actor
    (:then
      (bind _output_get (Variables|Default|SetPlayerVisible (.bsuccessfullysensed Stimulus)))
      (if _output_get
        _))
    (:CastFailed
      (Variables|Default|SetTargetPoint (.stimuluslocation Stimulus)))))

(event StateChangedDelegate(StateMachine)
  (params (NewStateTag :type Gameplay%20Tag%20Structure%20%28by%20ref%29)))

(event Custom|ScanningDone
  (bind _statemachine (Variables|Default|GetStateMachine))
  (if (GameplayTags|MatchesTag (Variables|/Script/StateMachine.StateMachineComponent|GetStateTag _statemachine) "(TagName=\"Defender.Alarmed.Scanning\")")
    (Class|StateMachineComponent|SwitchState _statemachine "(TagName=\"Defender.Alarmed.Returning\")")))

(event Custom|TargetReachedByPawn
  (bind _statemachine (Variables|Default|GetStateMachine))
  (if (GameplayTags|MatchesTag (Variables|/Script/StateMachine.StateMachineComponent|GetStateTag _statemachine) "(TagName=\"Defender.Alarmed.Returning\")")
    (Class|StateMachineComponent|SwitchState _statemachine "(TagName=\"Defender.Resting\")")
    (else
      (Class|StateMachineComponent|SwitchState _statemachine "(TagName=\"Defender.Alarmed.Scanning\")"))))

(event EventBeginPlay
  (bind _variables (Variables|Default|GetVariables))
  (bind _variables_2 (Variables|Default|GetVariables))
  (bind _rulestosleep (Variables|Default|GetRulesToSleep))
  (bind _rulestochase (Variables|Default|GetRulesToChase))
  (bind _rulestoattack (Variables|Default|GetRulesToAttack))
  (bind _outactors (Actor|GetAllActorsOfClass "/Game/Player/BP_Player.BP_Player_C"))
  (bind _asbp_player (Utilities|Casting|CastToBP_Player (Utilities|Array|Get(acopy) _outactors)))
  (Variables|Default|SetTargetPlayer _asbp_player)
  (Variables|Default|SetStartPoint (Transformation|GetActorLocation))
  ;[1 1 1] Нечёткая инициализация
  (bind _returnvalue (Game|ConstructObjectfromClass "/Script/FuzzyEngine.FVariable" self))
  (bind _output_get (Variables|Default|SetDistance _returnvalue))
  (Class|FVariable|AddTrapezoidTerm _output_get "Close" 0.0 0.0 1.5e+02 3e+02)
  (Class|FVariable|AddTrapezoidTerm _output_get "FarEnough" 1.5e+02 3e+02 7.5e+02 2e+03)
  (Class|FVariable|AddCrispTerm _output_get "TooFar" 1.5e+03 "MOQ")
  (bind _returnvalue_2 (Game|ConstructObjectfromClass "/Script/FuzzyEngine.FVariable" self))
  (bind _output_get_2 (Variables|Default|SetAwaken _returnvalue_2))
  (Class|FVariable|AddTriangularTerm _output_get_2 "Awaken" 0.0 25.0 5e+01)
  (Class|FVariable|AddTriangularTerm _output_get_2 "NotAwaken" 1e+01 6e+01 1e+02)
  (bind _returnvalue_3 (Game|ConstructObjectfromClass "/Script/FuzzyEngine.FVariable" self))
  (bind _output_get_3 (Variables|Default|SetAttackPlayer _returnvalue_3))
  (Class|FVariable|AddTrapezoidTerm _output_get_3 "Punch" 0.0 0.0 5.0 12.0)
  (Class|FVariable|AddCrispTerm _output_get_3 "NotPunch" 1e+01 "MOQ")
  (bind _returnvalue_4 (Game|ConstructObjectfromClass "/Script/FuzzyEngine.FEngine" self))
  (Variables|Default|SetFEngine _returnvalue_4)
  (bind _returnvalue_5 (Game|ConstructObjectfromClass "/Script/FuzzyEngine.TermSelector" self))
  (Variables|Default|SetTermSelector _returnvalue_5)
  ;[1 1 1] Тут добавляем переменные
  (Utilities|Map|Add _variables_2 "Awaken" (Variables|Default|GetAwaken))
  (Utilities|Map|Add _variables_2 "Distance" (Variables|Default|GetDistance))
  (Utilities|Map|Add _variables_2 "AttackPlayer" (Variables|Default|GetAttackPlayer))
  ;[1 1 1] Тут правила (много)
  (bind _returnvalue_6 (Class|RuleParser|ParseRuleString (Variables|Default|GetRuleToAwake) _variables))
  (Utilities|Array|Add _rulestosleep _returnvalue_6)
  (bind _returnvalue_7 (Class|RuleParser|ParseRuleString (Variables|Default|GetRuleToStaySleep) _variables))
  (Utilities|Array|Add _rulestosleep _returnvalue_7)
  (bind _returnvalue_8 (Class|RuleParser|ParseRuleString (Variables|Default|GetRuleToAttack) _variables))
  (Utilities|Array|Add _rulestoattack _returnvalue_8)
  (bind _returnvalue_9 (Class|RuleParser|ParseRuleString (Variables|Default|GetRuleToNotAttack) _variables))
  (Utilities|Array|Add _rulestoattack _returnvalue_9)
  (bind _returnvalue_10 (Class|RuleParser|ParseRuleString (Variables|Default|GetRuleToStopChasing) _variables))
  (Utilities|Array|Add _rulestochase _returnvalue_10)
  (bind _returnvalue_11 (Class|RuleParser|ParseRuleString (Variables|Default|GetRuleToChase) _variables))
  (Utilities|Array|Add _rulestochase _returnvalue_11))

(event EventTick
  (params (DeltaSeconds :type Float%20%28single-precision%29))
  (bind _targetplayer (Variables|Default|GetTargetPlayer))
  (Utilities|FlowControl|Delay 0.2)
  (if (Utilities|IsValid _targetplayer)
    (Class|FVariable|SetInput (Variables|Default|GetDistance) (Math|Vector|Distance(Vector) (Transformation|GetActorLocation _targetplayer) (Transformation|GetActorLocation (Pawn|GetControlledPawn))))))

(event EventPossess
  (params (PossessedPawn :type Pawn%20Object%20Reference))
  (bind _asbp_defender (Utilities|Casting|CastToBP_Defender PossessedPawn))
  (bind _output_get (Variables|Default|SetAs%20BP%20Defender _asbp_defender))
  (Variables|Default|SetStartPoint (Transformation|GetActorLocation _output_get))
  (EventDispatchers|BindEventtoScanningIsOver _output_get (delegate Custom|ScanningDone))
  (EventDispatchers|BindEventtoTargetReached _output_get (delegate Custom|TargetReachedByPawn))
  (AI|RunBehaviorTree "/Game/Pawns/Defender/BT_Defender.BT_Defender"))

(fn ConstructionScript)

(fn StartResting
  (Default|PlayAnimation (Variables|Default|GetAs%20BP%20Defender) "/Game/RamsterZ_FreeAnims_Volume1/AnimationSequence/H2H/H2H_Idle.H2H_Idle" true))

(fn KillPlayer
  (bind _as_bp_defender (Variables|Default|GetAs%20BP%20Defender))
  (bind _statemachine (Variables|Default|GetStateMachine))
  (if (Utilities|IsValid (Variables|Default|GetTargetPlayer))
    (Default|PlayAnimation _as_bp_defender "/Game/RamsterZ_FreeAnims_Volume1/AnimationSequence/H2H/H2H_Kick01.H2H_Kick01" false)
    (if (< (Class|FVariable|GetInput (Variables|Default|GetDistance)) (Variables|/Game/Pawns/Defender/BP_Defender.BP_Defender_C|GetDistanceToKill _as_bp_defender))
      (Default|Die (Variables|Default|GetTargetPlayer))
      (Class|StateMachineComponent|SwitchState _statemachine "(TagName=\"Defender.Resting\")")
      (Variables|Default|SetTargetPlayer 0)
      (else
        (Class|StateMachineComponent|SwitchState _statemachine "(TagName=\"Defender.Aggression.Chasing\")")))))

(fn RuntoTarget
  (AI|Navigation|SimpleMovetoLocation self (Variables|Default|GetTargetPoint))
  (Variables|/Game/Pawns/Defender/BP_Defender.BP_Defender_C|SetTargetPoint (Variables|Default|GetAs%20BP%20Defender) (Variables|Default|GetTargetPoint)))

(fn ChasePlayer
  (AI|Navigation|MovetoActor (Variables|Default|GetTargetPlayer) -1.0 true true true 0))